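; bp_funcs is a shared function collection with a debug print helper and a look-at check for interactable actors.
; Debugger prints a title joined to a value when its condition is true.
; Looker sphere-traces on the Visibility channel along a camera's forward vector for a given distance.
; It returns the hit actor and true only if that actor implements I_interact, otherwise None and false.
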(fn `debugger`
  (params (Title :type String) (Var :type String) (condition :type Boolean))
  (if condition
    (`KismetSystemLibrary.PrintString` null (`KismetStringLibrary.Concat_StrStr` Title Var) true true (struct :`G` 0.66 :`B` 1.0 :`A` 1.0) 0.0)))

(fn `looker`
  (params (WorldContextObject :type "Object Object Reference") (camera :type "SceneComponent Object Reference") (lookDistance :type "Float (double-precision)"))
  (returns (a_hitActor1 :type "Actor Object Reference") (b_hitInterface1 :type Boolean))
  (locals (b_hitInterface :type Boolean) (a_hitActor :type "Actor Object Reference"))
  (bind _returnvalue (`SceneComponent.K2_GetComponentLocation` camera))
  (bind (_outhit _returnvalue_2) (`KismetSystemLibrary.SphereTraceSingle` :`WorldContextObject` WorldContextObject :`Start` _returnvalue :`End` (+ _returnvalue (* (`KismetMathLibrary.GetForwardVector` (`SceneComponent.K2_GetComponentRotation` camera)) lookDistance)) :`Radius` 5.0 :`TraceChannel` "TraceTypeQuery1" :`bTraceComplex` true :`DrawTime` 0.1))
  (if _returnvalue_2
    (bind (_bblockinghit _binitialoverlap _time _distance _location _impactpoint _normal _impactnormal _physmat _hitactor) (`GameplayStatics.BreakHitResult` _outhit))
    (if (`KismetSystemLibrary.DoesImplementInterface` _hitactor "/Game/Interfaces/i_interact.i_interact_C")
      (set `local.b_hitInterface` true)
      (set `local.a_hitActor` _hitactor)
      (else
        (set `local.b_hitInterface` false :!label _label)
        (set `local.a_hitActor` null)))
    (else
      (goto _label)))
  (return (`local.a_hitActor`) (`local.b_hitInterface`)))